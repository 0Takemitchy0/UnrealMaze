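; BP_BlueDoor is a door that opens when a key of the matching color is collected.
; Its CollectKey event compares the passed material to the Cube's first material and, on a match, plays a timeline that lowers the Cube along relative Z.
; CatchDoorColorByName and CatchKeyColorByName hold unused logic for parsing color names from object names, so matching relies on material alone.
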(event `/Game/dosya/Blueprints/Interfaces/BPI_DoorsNKeys.CollectKey`
  (params (Material :type "MaterialInterface Object Reference"))
  (if (== Material (`PrimitiveComponent.GetMaterial` (`self.Cube`) 0))
    (bind (_direction _opendoor) (`Timeline|Open Timeline`)
      (:`Update`
        (`SceneComponent.K2_SetRelativeLocation` (`self.Cube`) (`KismetMathLibrary.MakeVector` 0.0 0.0 (`KismetMathLibrary.Lerp` 0.0 -500.0 _opendoor)) false false)))))

(fn `UserConstructionScript`)