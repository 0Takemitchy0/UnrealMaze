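; BP_Door2 is a door that slides down once it has been triggered twice.
; Each kapıçek event increments the Say counter; on the second, OpenTimeline lerps the Cube's relative Z downward to open it.
; CollectKey compares a key material to the Cube's but does nothing with the result.
; CatchDoorColorByName and CatchKeyColorByName hold only unused string splits for parsing object names.
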(event `self.CollectKey`
  (params (Material :type "MaterialInterface Object Reference"))
  (if (== Material (`PrimitiveComponent.GetMaterial` (`self.Cube`) 0))
    _))

(event `kapıçek`
  (`/Engine/EditorBlueprintResources/StandardMacros.IncrementInt` (`self.say`)
    (:`  `
      (if (== (`self.say`) 2)
        (bind (_direction _opendoor) (`Timeline|Open Timeline`)
          (:`Update`
            (`SceneComponent.K2_SetRelativeLocation` (`self.Cube`) (`KismetMathLibrary.MakeVector` 0.0 0.0 (`KismetMathLibrary.Lerp` 0.0 -500.0 _opendoor)) false false)))))))

(fn `UserConstructionScript`)