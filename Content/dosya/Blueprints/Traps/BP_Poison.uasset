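; BP_Poison is a trap area that deals repeated damage to the player until levers deactivate it.
; Box begin overlap starts a looping damage timer through a NAND of player and deactivated checks, so other actors also trigger it.
; The timer calls the player's DamageFunction, and the player leaving the box clears it.
; It binds to every BP_TrapLever's poison dispatcher, which sets the flag and destroys the actor.
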(event `self.ReceiveBeginPlay`
  (bind _asbp_third_person_character (cast `/Game/ThirdPerson/Blueprints/BP_ThirdPersonCharacter` (`GameplayStatics.GetPlayerCharacter` 0)))
  (set `self.Player` _asbp_third_person_character)
  (bind _outactors (`GameplayStatics.GetAllActorsOfClass` "/Game/dosya/Blueprints/Traps/BP_TrapLever.BP_TrapLever_C"))
  (bind _output_get (set `self.Levers` _outactors))
  (add `/Game/dosya/Blueprints/Traps/BP_TrapLever.DP_Poison` _output_get (delegate `DP_Poison_Event`)))

(event `DP_Poison_Event`
  (params (DeactivatePoison :type Boolean))
  (set `self.IsDeactivated` DeactivatePoison)
  (`KismetSystemLibrary.PrintString` "Poisonous areas are deactivated")
  (`self.K2_DestroyActor`))

(event `self.Box.OnComponentBeginOverlap`
  (params (OverlappedComponent :type "PrimitiveComponent Object Reference") (OtherActor :type "Actor Object Reference") (OtherComp :type "PrimitiveComponent Object Reference") (OtherBodyIndex :type Integer) (bFromSweep :type Boolean) (SweepResult :type "HitResult Structure (by ref)"))
  (if (`KismetMathLibrary.BooleanNAND` (== OtherActor (`self.Player`)) (`self.IsDeactivated`))
    (bind _returnvalue (`KismetSystemLibrary.K2_SetTimerDelegate` (delegate `Apply Damage on Time`) 0.33 true))
    (set `self.Timer` _returnvalue)))

(event `Apply Damage on Time`
  (`/Game/ThirdPerson/Blueprints/BP_ThirdPersonCharacter.Damage Function` (`self.Player`) (`self.Damage`)))

(event `self.Box.OnComponentEndOverlap`
  (params (OverlappedComponent :type "PrimitiveComponent Object Reference") (OtherActor :type "Actor Object Reference") (OtherComp :type "PrimitiveComponent Object Reference") (OtherBodyIndex :type Integer))
  (if (== OtherActor (`self.Player`))
    (`KismetSystemLibrary.K2_ClearAndInvalidateTimerHandle` (`self.Timer`))))

(fn `UserConstructionScript`)