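; BP_Spike is a spike trap that damages the player character on contact with its DamageGiver collider.
; Box overlap plays the LaunchSpikes timeline to move the spikes, reversing it when the player leaves.
; It binds to every BP_TrapLever's DPSpike dispatcher to set IsDeactivated.
; The launch check uses NAND, so non-player actors always trigger it and deactivation only blocks the player's trigger, without disabling damage.
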(event `self.ReceiveBeginPlay`
  (bind _asbp_third_person_character (cast `/Game/ThirdPerson/Blueprints/BP_ThirdPersonCharacter` (`GameplayStatics.GetPlayerCharacter` 0)))
  (set `self.Player` _asbp_third_person_character)
  (bind _outactors (`GameplayStatics.GetAllActorsOfClass` "/Game/dosya/Blueprints/Traps/BP_TrapLever.BP_TrapLever_C"))
  (bind _output_get (set `self.Levers` _outactors))
  (add `/Game/dosya/Blueprints/Traps/BP_TrapLever.DP_Spike` _output_get (delegate `DP_Spike_Event`)))

(event `DP_Spike_Event`
  (params (DeactiveSpike :type Boolean))
  (set `self.IsDeactivated` DeactiveSpike)
  (`KismetSystemLibrary.PrintString` "Spikes are deactivated"))

(event `self.Box.OnComponentBeginOverlap`
  (params (OverlappedComponent :type "PrimitiveComponent Object Reference") (OtherActor :type "Actor Object Reference") (OtherComp :type "PrimitiveComponent Object Reference") (OtherBodyIndex :type Integer) (bFromSweep :type Boolean) (SweepResult :type "HitResult Structure (by ref)"))
  (if (`KismetMathLibrary.BooleanNAND` (== OtherActor (`self.Player`)) (`self.IsDeactivated`))
    (bind (_direction _z) (`Timeline|Launch Spikes` :!label _label)
      (:`Update`
        (`SceneComponent.K2_SetRelativeLocation` (`self.Spike`) (`KismetMathLibrary.MakeVector` 1.5 1.5 _z) false false)))))

(event `self.Box.OnComponentEndOverlap`
  (params (OverlappedComponent :type "PrimitiveComponent Object Reference") (OtherActor :type "Actor Object Reference") (OtherComp :type "PrimitiveComponent Object Reference") (OtherBodyIndex :type Integer))
  (if (== OtherActor (`self.Player`))
    (goto _label :!via `Reverse`)))

(event `self.DamageGiver.OnComponentBeginOverlap`
  (params (OverlappedComponent :type "PrimitiveComponent Object Reference") (OtherActor :type "Actor Object Reference") (OtherComp :type "PrimitiveComponent Object Reference") (OtherBodyIndex :type Integer) (bFromSweep :type Boolean) (SweepResult :type "HitResult Structure (by ref)"))
  (if (== OtherActor (`self.Player`))
    (`/Game/ThirdPerson/Blueprints/BP_ThirdPersonCharacter.Damage Function` (`self.Player`) (`self.Damage`))))

(fn `UserConstructionScript`)