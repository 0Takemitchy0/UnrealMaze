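; BP_Xp is an experience pickup that homes in on the player and grants XP on contact.
; On BeginPlay it caches the player's BP_ThirdPersonCharacter.
; A Sphere overlap plays the Lerp timeline, which pulls the actor from its current location toward the player's live location while the overlapping actor is the player.
; A Cube overlap with the player calls AddXp and destroys the pickup.
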(event `self.Cube.OnComponentBeginOverlap`
  (params (OverlappedComponent :type "PrimitiveComponent Object Reference") (OtherActor :type "Actor Object Reference") (OtherComp :type "PrimitiveComponent Object Reference") (OtherBodyIndex :type Integer) (bFromSweep :type Boolean) (SweepResult :type "HitResult Structure (by ref)"))
  (if (== OtherActor (`self.Player`))
    (`/Game/ThirdPerson/Blueprints/BP_ThirdPersonCharacter.Add Xp` (`self.Player`))
    (`self.K2_DestroyActor`)))

(event `self.Sphere.OnComponentBeginOverlap`
  (params (OverlappedComponent :type "PrimitiveComponent Object Reference") (OtherActor :type "Actor Object Reference") (OtherComp :type "PrimitiveComponent Object Reference") (OtherBodyIndex :type Integer) (bFromSweep :type Boolean) (SweepResult :type "HitResult Structure (by ref)"))
  (bind _player (`self.Player`))
  (bind (_direction _lerp) (`Timeline|Lerp`)
    (:`Update`
      (if (== OtherActor _player)
        (`self.K2_SetActorLocation` self (`KismetMathLibrary.VLerp` (`self.K2_GetActorLocation` self) (`self.K2_GetActorLocation` _player) _lerp) false false)))))

(event `self.ReceiveBeginPlay`
  (bind _asbp_third_person_character (cast `/Game/ThirdPerson/Blueprints/BP_ThirdPersonCharacter` (`GameplayStatics.GetPlayerCharacter` 0)))
  (set `self.Player` _asbp_third_person_character))

(fn `UserConstructionScript`)