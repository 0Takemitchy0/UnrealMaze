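; BP_Gold is a gold pickup with a random value that the player collects by touching it.
; The construction script rolls the value and adds one, two or three differently scaled static meshes, so richer pickups look bigger.
; When the cached player character overlaps the sphere, the pickup passes its value through CollectGoldMessage and destroys itself.
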(event `self.ReceiveBeginPlay`
  (bind _asbp_third_person_character (cast `/Game/ThirdPerson/Blueprints/BP_ThirdPersonCharacter` (`GameplayStatics.GetPlayerCharacter` 0)))
  (set `self.Player` _asbp_third_person_character))

(event `self.Sphere.OnComponentBeginOverlap`
  (params (OverlappedComponent :type "PrimitiveComponent Object Reference") (OtherActor :type "Actor Object Reference") (OtherComp :type "PrimitiveComponent Object Reference") (OtherBodyIndex :type Integer) (bFromSweep :type Boolean) (SweepResult :type "HitResult Structure (by ref)"))
  (if (== OtherActor (`self.Player`))
    (message `/Game/dosya/Blueprints/Interfaces/BPI_DoorsNKeys.CollectGold` OtherActor (`self.Value`))
    (`self.K2_DestroyActor`)))

(fn `UserConstructionScript`
  (bind _output_get (set `self.Value` (`KismetMathLibrary.RandomIntegerInRange` 1 99)))
  (if (>= _output_get 76)
    (`|ExecutionSequence`
      (:`then_0`
        (`AddComponent|NODE_AddStaticMeshComponent-0` :`RelativeTransform` (`KismetMathLibrary.MakeTransform` (-50.0 -50.0 0.0))))
      (:`then_1`
        (`AddComponent|NODE_AddStaticMeshComponent-1` :`RelativeTransform` (`KismetMathLibrary.MakeTransform` (-25.0 50.0 0.0) (struct) (0.7 0.7 0.7)) :!label _label))
      (:`then_2`
        (`AddComponent|NODE_AddStaticMeshComponent-2` :`RelativeTransform` (`KismetMathLibrary.MakeTransform` (50.0 0.0 0.0) (struct) (0.45 0.45 0.45)) :!label _label_2)))
    (elif (>= _output_get 26)
      (`|ExecutionSequence`
        (:`then_0`
          (goto _label))
        (:`then_1`
          (goto _label_2)))
      (else
        (goto _label_2)))))